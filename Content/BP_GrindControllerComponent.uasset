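; Grind controller component that slides the player character along a rail spline from its landing point.
; Grind locks movement, overlaps WorldStatic and picks travel direction from facing versus spline yaw.
; A constructed SimplifiedTimeline drives interpolated capsule position along the spline, aligns yaw and tilts the mesh with slope.
; Reaching the end or pressing Space launches the character by input or facing, higher when jumping, then restores movement and collision.
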(event `Jump From Rail`
  (bind _rcrcharacter (`self.RCRCharacter`))
  (bind _rcrcharacter_2 (`self.RCRCharacter`))
  (bind _returnvalue (`Actor.K2_GetActorRotation` (`self.RCRCharacter`)))
  (bind (_movementinputvector_x _movementinputvector_y) (`KismetMathLibrary.BreakVector2D` (`RhythmCityRushCharacter.MovementInputVector` (`self.RCRCharacter`))))
  (bind (_movementinputvector_x_2 _movementinputvector_y_2) (`KismetMathLibrary.BreakVector2D` (`RhythmCityRushCharacter.MovementInputVector` (`self.RCRCharacter`))))
  (bind (_returnvalue_x _returnvalue_y) (`KismetMathLibrary.BreakVector` (`SceneComponent.GetForwardVector` (`Character.CapsuleComponent` (`self.RCRCharacter`)))))
  (bind _returnvalue_2 (* _returnvalue_x 500.0))
  (bind _returnvalue_3 (* _returnvalue_y 500.0))
  (bind (_returnvalue_x_2 _returnvalue_y_2) (`KismetMathLibrary.BreakVector` (+ (* (`KismetMathLibrary.GetForwardVector` _returnvalue) _movementinputvector_y) (* (`KismetMathLibrary.GetRightVector` _returnvalue) _movementinputvector_x))))
  (bind _returnvalue_4 (* _returnvalue_x_2 500.0))
  (bind _returnvalue_5 (* _returnvalue_y_2 500.0))
  ;[1 1 1] When jumping from the Rail, the character is launched depending on the directional input or if the Player is holding any directional input at all. Then stops the Rail sound effect, detaches and destroys the speedlines. If a Montage was playing, it is stopped. Sets the normal relative rotation of the Skeletal Mesh. After a short delay the character can move again and we set the Capsule collision to Block WorldStatic again
  (if (and (== _movementinputvector_x_2 0.0) (== _movementinputvector_y_2 0.0))
    (if (`self.bJumpedWhileGrinding`)
      (`Character.LaunchCharacter` _rcrcharacter (`KismetMathLibrary.MakeVector` _returnvalue_2 _returnvalue_3 550.0) false true)
      (else
        (`Character.LaunchCharacter` _rcrcharacter (`KismetMathLibrary.MakeVector` _returnvalue_2 _returnvalue_3 100.0) false true)))
    (elif (`self.bJumpedWhileGrinding`)
      (`Character.LaunchCharacter` _rcrcharacter_2 (`KismetMathLibrary.MakeVector` _returnvalue_4 _returnvalue_5 550.0) false true)
      (else
        (`Character.LaunchCharacter` _rcrcharacter_2 (`KismetMathLibrary.MakeVector` _returnvalue_4 _returnvalue_5 100.0) false true))))
  (set `self.Rail Spline` null)
  (set `self.bJumpedWhileGrinding` false)
  (`SceneComponent.K2_SetRelativeRotation` (`Character.Mesh` (`self.RCRCharacter`)) (struct :`Yaw` -90.0) false false)
  (`KismetSystemLibrary.Delay` 0.1)
  (`RhythmCityRushCharacter.SetCanMove` (`self.RCRCharacter`) true)
  (`PrimitiveComponent.SetCollisionResponseToChannel` (`Character.CapsuleComponent` (`self.RCRCharacter`)) "ECC_WorldStatic" "ECR_Block"))

(event `OnTimerFinished_Event`
  (params (CurrentValue :type "Float (single-precision)") (Direction :type "ESimplifiedTimelineDirection Enum" :default "Forward"))
  ;[1 1 1] When jumping from the Rail, the character is launched depending on the directional input or if the Player is holding any directional input at all. Then stops the Rail sound effect, detaches and destroys the speedlines. If a Montage was playing, it is stopped. Sets the normal relative rotation of the Skeletal Mesh. After a short delay the character can move again and we set the Capsule collision to Block WorldStatic again
  (set `self.bIsPlayingGrindTimeline` false)
  (`|ExecutionSequence`
    (:`then_0`
      (`SimplifiedTimeline.Stop` (`self.SimplifiedGrindTimeline`)))
    (:`then_1`
      (`self.Jump From Rail`))))

(event `self.ReceiveBeginPlay`
  (bind _simplifiedgrindtimeline (`self.SimplifiedGrindTimeline`))
  (bind _returnvalue (`|GenericCreateObject` self "/Script/RhythmCityRush.SimplifiedTimeline" 60.0 "/Game/GrindTimelineCurve.GrindTimelineCurve"))
  (set `self.SimplifiedGrindTimeline` _returnvalue)
  (add `SimplifiedTimeline.OnTimerUpdate` _simplifiedgrindtimeline (delegate `OnTimerUpdate_Event`))
  (add `SimplifiedTimeline.OnTimerFinished` _simplifiedgrindtimeline (delegate `OnTimerFinished_Event`)))

(event `Key|SpaceBar`
  (params (Key :type "Key Structure"))
  ;[1 1 1] Handle jumping while grinding
  (:`Pressed`
    (if (`self.bIsPlayingGrindTimeline`)
      (set `self.bJumpedWhileGrinding` true)
      (`SimplifiedTimeline.SkipToEnd` (`self.SimplifiedGrindTimeline`)))))

(event `OnTimerUpdate_Event`
  (params (CurrentValue :type "Float (single-precision)") (Direction :type "ESimplifiedTimelineDirection Enum" :default "Forward"))
  (bind _rail_spline (`self.Rail Spline`))
  (bind _rail_spline_2 (`self.Rail Spline`))
  (bind _relativerotation_roll (`KismetMathLibrary.BreakRotator` (`SceneComponent.RelativeRotation` (`Character.Mesh` (`self.RCRCharacter`)))))
  (bind _returnvalue (`KismetMathLibrary.Lerp` (`SplineComponent.GetDistanceAlongSplineAtSplineInputKey` _rail_spline_2 (`SplineComponent.FindInputKeyClosestToWorldLocation` _rail_spline_2 (`SplineComponent.FindLocationClosestToWorldLocation` _rail_spline_2 (`self.RailLandingLocation`) "World"))) (`KismetMathLibrary.SelectFloat` (`SplineComponent.GetSplineLength` (`self.Rail Spline`)) 0.0 (`self.ForwardDirection`)) CurrentValue))
  (bind (_returnvalue_roll _returnvalue_pitch _returnvalue_yaw) (`KismetMathLibrary.BreakRotator` (`SplineComponent.GetRotationAtDistanceAlongSpline` _rail_spline _returnvalue "World")))
  (bind _returnvalue_2 (`KismetMathLibrary.NormalizeAxis` _returnvalue_pitch))
  (set `self.bIsPlayingGrindTimeline` true)
  (`SceneComponent.K2_SetWorldLocationAndRotation` (`Character.CapsuleComponent` (`self.RCRCharacter`)) (`KismetMathLibrary.VInterpTo` (`SceneComponent.K2_GetComponentLocation` (`Character.CapsuleComponent` (`self.RCRCharacter`))) (+ (`SplineComponent.GetLocationAtDistanceAlongSpline` _rail_spline _returnvalue "World") (0.0 0.0 135.0)) (`GameplayStatics.GetWorldDeltaSeconds`) 80.0) (`KismetMathLibrary.MakeRotator` 0.0 0.0 (select `bool` (`self.ForwardDirection`) :`false` (select `bool` (>= (`KismetMathLibrary.NormalizeAxis` _returnvalue_yaw) 0.0) :`false` (+ _returnvalue_yaw 180.0) :`true` (- _returnvalue_yaw 180.0)) :`true` _returnvalue_yaw :!type "Float (double-precision)")) true false)
  (`SceneComponent.K2_SetRelativeRotation` (`Character.Mesh` (`self.RCRCharacter`)) (`KismetMathLibrary.MakeRotator` (`KismetMathLibrary.FInterpTo` _relativerotation_roll (select `bool` (`self.ForwardDirection`) :`false` _returnvalue_2 :`true` (* _returnvalue_2 -1.0) :!type "Float (double-precision)") (`GameplayStatics.GetWorldDeltaSeconds`) 20.0) 0.0 -90.0) false false))

(event `self.Grind`
  (params (LandingHit :type "HitResult Structure") (RailSpline :type "SplineComponent Object Reference") (PlayerChar :type "RhythmCityRushCharacter Object Reference"))
  (bind _rail_spline (`self.Rail Spline`))
  (bind _returnvalue (`SplineComponent.GetSplineLength` (`self.Rail Spline`)))
  (bind _returnvalue_2 (`SplineComponent.GetDistanceAlongSplineAtSplineInputKey` _rail_spline (`SplineComponent.FindInputKeyClosestToWorldLocation` _rail_spline (`SplineComponent.FindLocationClosestToWorldLocation` _rail_spline (`self.RailLandingLocation`) "World"))))
  (set `self.Rail Spline` RailSpline)
  (set `self.RCRCharacter` PlayerChar)
  (set `self.RawRailSpeed` (/ (* (`SplineComponent.GetSplineLength` (`self.Rail Spline`)) (`self.RawRailSpeedMultiplier`)) 1000.0))
  (`RhythmCityRushCharacter.SetCanMove` (`self.RCRCharacter`) false)
  (set `self.RailLandingLocation` (`.ImpactPoint` (`GameplayStatics.BreakHitResult` LandingHit)))
  (set `self.ForwardDirection` (or (`self.SimilarRotation` 90.0) (`self.SimilarRotation` -90.0)))
  (set `self.SpeedWithoutBonus` (`KismetMathLibrary.SelectFloat` (/ (* (`self.RawRailSpeed`) (- _returnvalue _returnvalue_2)) _returnvalue) (/ (* (`self.RawRailSpeed`) _returnvalue_2) (`SplineComponent.GetSplineLength` (`self.Rail Spline`))) (`self.ForwardDirection`)))
  (set `SimplifiedTimeline.PlaybackFrequency` 1250.0 (`self.SimplifiedGrindTimeline`))
  (`PrimitiveComponent.SetCollisionResponseToChannel` (`Character.CapsuleComponent` (`self.RCRCharacter`)) "ECC_WorldStatic" "ECR_Overlap")
  (`SimplifiedTimeline.Play` (`self.SimplifiedGrindTimeline`)))

(fn `SimilarRotation`
  (params (`Z var` :type "Float (double-precision)"))
  (returns (`In Range?` :type Boolean))
  (bind _rail_spline (`self.Rail Spline`))
  (bind (_returnvalue_roll _returnvalue_pitch _returnvalue_yaw) (`KismetMathLibrary.BreakRotator` (`SceneComponent.K2_GetComponentRotation` (`Character.CapsuleComponent` (`self.RCRCharacter`)))))
  (bind (_returnvalue_roll_2 _returnvalue_pitch_2 _returnvalue_yaw_2) (`KismetMathLibrary.BreakRotator` (`SplineComponent.GetRotationAtDistanceAlongSpline` _rail_spline (`SplineComponent.GetDistanceAlongSplineAtSplineInputKey` _rail_spline (`SplineComponent.FindInputKeyClosestToWorldLocation` _rail_spline (`SplineComponent.FindLocationClosestToWorldLocation` _rail_spline (`self.RailLandingLocation`) "World"))) "World")))
  (bind _returnvalue (+ _returnvalue_yaw_2 `Z var`))
  (bind _returnvalue_2 (`KismetMathLibrary.NormalizeAxis` _returnvalue))
  (bind _returnvalue_3 (`KismetMathLibrary.NearlyEqual_FloatFloat` _returnvalue _returnvalue_2 0.1))
  (bind _returnvalue_4 (> _returnvalue_yaw_2 _returnvalue_2))
  (bind _returnvalue_5 (select `bool` _returnvalue_3 :`true` true))
  (bind _returnvalue_6 (`KismetMathLibrary.InRange_FloatFloat` _returnvalue_yaw (`KismetMathLibrary.SelectFloat` _returnvalue_2 _returnvalue_yaw_2 _returnvalue_4) (`KismetMathLibrary.SelectFloat` _returnvalue_yaw_2 _returnvalue_2 _returnvalue_4) _returnvalue_5 _returnvalue_5))
  (return (select `bool` _returnvalue_3 :`false` (not _returnvalue_6) :`true` _returnvalue_6)))

(fn `UpdateTimelinePlayRate`
  (bind _onrailspeed (`self.OnRailSpeed`))
  (set `self.OnRailSpeed` (- (`self.SpeedWithoutBonus`) (/ (* (`self.SpeedWithoutBonus`) (`self.TotalSpeedBonus`)) 100.0)))
  (set `SimplifiedTimeline.PlaybackFrequency` (/ 1.0 (`KismetMathLibrary.SelectFloat` 0.1 _onrailspeed (<= _onrailspeed 0.0))) (`self.SimplifiedGrindTimeline`)))

(fn `UserConstructionScript`)